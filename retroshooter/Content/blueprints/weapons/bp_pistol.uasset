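; Pistol weapon Blueprint that plays 2D flipbook animations and sounds when the player shoots.
; Shootweapon passes a DoOnce gate, calls Fireweapon, then reads Ammo by casting itself to bp_BaseWeapon.
; Zero ammo plays a punch animation and sound; otherwise it plays pistol fire.
; After a delay matching the flipbook length, it restores the matching idle flipbook and resets the gate.
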(event Custom|resetweapon
  (bind _weaponfliperbook (Variables|Default|GetWeaponfliperbook))
  (bind _weaponfliperbook_2 (Variables|Default|GetWeaponfliperbook))
  (Utilities|FlowControl|DoOnce false) ; enters at Reset
)

(event EventBeginPlay
  (|CallParentFunction) ; This node is disabled and will not be called.\nDrag off pins to build functionality.
)

(event Collision|EventActorBeginOverlap
  (params (OtherActor :type Actor%20Object%20Reference))
  (|CallParentFunction OtherActor) ; This node is disabled and will not be called.\nDrag off pins to build functionality.
)

(event EventTick
  (params (DeltaSeconds :type Float%20%28single-precision%29))
  (|CallParentFunction DeltaSeconds) ; This node is disabled and will not be called.\nDrag off pins to build functionality.
)

(event EventShootweapon
  (bind _weaponfliperbook (Variables|Default|GetWeaponfliperbook))
  (bind _weaponfliperbook_2 (Variables|Default|GetWeaponfliperbook))
  (Utilities|FlowControl|DoOnce false
    (:Completed
      (CallFunction|Fireweapon)
      (bind _asbp_base_weapon (Utilities|Casting|CastTobp_BaseWeapon self))
      (if (== (Variables|/Game/blueprints/weapons/bp_BaseWeapon.bp_BaseWeapon_C|GetAmmo _asbp_base_weapon) 0)
        (Sprite|SetFlipbook _weaponfliperbook "/Game/sprites/Weapons/Punch/punch.punch")
        (Audio|PlaySound2D "/Game/Sounds/014_Ooof.014_Ooof" 1.0 1.0 0.0 0 0)
        (Utilities|FlowControl|Delay (Class|PaperFlipbookComponent|GetFlipbookLength _weaponfliperbook))
        (Sprite|SetFlipbook (Variables|Default|GetWeaponfliperbook) "/Game/sprites/Weapons/Punch/punchidle.punchidle")
        (CallFunction|Resetweapon)
        (else
          (Sprite|SetFlipbook _weaponfliperbook_2 "/Game/sprites/Weapons/Pistol/pistolfire.pistolfire")
          (Audio|PlaySound2D "/Game/Sounds/005_PlayerPistol.005_PlayerPistol" 1.0 1.0 0.0 0 0)
          (Utilities|FlowControl|Delay (Class|PaperFlipbookComponent|GetFlipbookLength _weaponfliperbook_2))
          (Sprite|SetFlipbook (Variables|Default|GetWeaponfliperbook) "/Game/sprites/Weapons/Pistol/pistolidle.pistolidle")
          (CallFunction|Resetweapon))))))

(fn ConstructionScript
  (|CallParentFunction))