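; Base weapon Blueprint that provides hitscan firing, with empty shoot and stop-shooting events, presumably for child weapons to override.
; Fireweapon prints and spends ammo, then line traces forward from the Linetrace component and applies weapon damage to the hit actor.
; With no ammo, it overwrites the trace distance with a short fixed range and still deals damage, without restoring the distance here.
; Both traces draw debug lines.
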(event Custom|shootweapon)

(event Custom|stopshooting)

(event EventBeginPlay)

(fn ConstructionScript)

(fn Fireweapon
  (bind _linetrace (Variables|Default|Getlinetrace))
  (bind _linetrace_2 (Variables|Default|Getlinetrace))
  (bind _returnvalue (Transformation|GetWorldLocation _linetrace))
  (bind _returnvalue_2 (Transformation|GetWorldLocation _linetrace_2))
  (if (== 0 (Variables|Default|GetAmmo))
    (Variables|Default|SetHaveAmmo false))
  (Development|PrintString (Utilities|String|ToString(Integer) (Variables|Default|GetAmmo)))
  (if (Variables|Default|GetHaveAmmo)
    (Variables|Default|SetAmmo (- (Variables|Default|GetAmmo) 1))
    (bind (_outhit _returnvalue_3) (Collision|LineTraceForObjects _returnvalue_2 (+ _returnvalue_2 (* (Math|Vector|GetForwardVector (Transformation|GetWorldRotation (Variables|Default|Getlinetrace))) (Variables|Default|Getlinetracedistance))) (Utilities|Array|MakeArray "ObjectTypeQuery1" "ObjectTypeQuery2" "ObjectTypeQuery3") false (Utilities|Array|MakeArray self (Game|GetPlayerCharacter 0)) "ForDuration"))
    (if _returnvalue_3
      (Game|Damage|ApplyDamage (.HitActor (Collision|BreakHitResult _outhit)) (Variables|Default|Getweapondmg) 0 0))
    (else
      (bind _output_get (Variables|Default|Setlinetracedistance 1e+02))
      (bind (_outhit_2 _returnvalue_4) (Collision|LineTraceForObjects _returnvalue (+ _returnvalue (* (Math|Vector|GetForwardVector (Transformation|GetWorldRotation (Variables|Default|Getlinetrace))) _output_get)) (Utilities|Array|MakeArray "ObjectTypeQuery1" "ObjectTypeQuery2" "ObjectTypeQuery3") false (Utilities|Array|MakeArray (Game|GetPlayerCharacter 0) 0) "ForDuration"))
      (if _returnvalue_4
        (Game|Damage|ApplyDamage (.HitActor (Collision|BreakHitResult _outhit_2)) (Variables|Default|Getweapondmg) 0 0)))))