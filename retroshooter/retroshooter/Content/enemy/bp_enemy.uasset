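; Sprite-based enemy character that roams randomly until PawnSensing spots the player, with Paper2D flipbooks showing movement, attack and death.
; AttackType picks the response: ranged enemies turn, spawn a projectile and also damage the player directly, while others chase via AIMoveTo and deal damage on arrival.
; The first damage of any amount kills it, stopping movement, playing death flipbooks, then setting Isdead and disabling capsule collision.
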(event OnSeePawn(PawnSensing)
  (params (Pawn :type Pawn%20Object%20Reference))
  (Variables|Default|SetIsAttacking true)
  (if (Utilities|String|Contains (Variables|Default|GetAttackType) "Ranged")
    ;[1 1 1] Attack
    (bind _asbp_first_person_character (Utilities|Casting|CastToBP_FirstPersonCharacter Pawn))
    (Transformation|SetActorRotation (Math|Rotator|FindRelativeLookatRotation (Math|Conversions|ToTransform(Vector) (Transformation|GetActorLocation)) (Transformation|GetActorLocation _asbp_first_person_character)))
    (if (Variables|Default|GetCanAttack)
      (if (not (Variables|Default|Getisdead))
        (Sprite|SetFlipbook (Variables|Default|GetPaperFlipbook) "/Game/enemy/RangedAttackFlip.RangedAttackFlip")
        (Game|SpawnActorfromClass "/Game/FirstPerson/Blueprints/BP_Projectile.BP_Projectile_C" (Transformation|GetWorldTransform (Variables|Default|GetBulletSpawnLocation)) "Undefined" "MultiplyWithRoot" 0 0 :!label _label)
        (bind _asbp_first_person_character_2 (Utilities|Casting|CastToBP_FirstPersonCharacter (Game|GetPlayerCharacter 0)))
        (Game|Damage|ApplyDamage _asbp_first_person_character_2 5.0 0 0)
        (Variables|Default|SetCanAttack false)
        (Utilities|FlowControl|Delay 0.5)
        (Variables|Default|SetCanAttack true))
      (else
        (Sprite|SetFlipbook (Variables|Default|GetPaperFlipbook) "/Game/sprites/Soldierwalksprie/SoldierMove.SoldierMove")
        (goto _label)))
    (else
      ;[1 1 1] Move To Player
      (bind _asbp_first_person_character_3 (Utilities|Casting|CastToBP_FirstPersonCharacter Pawn))
      (Variables|Default|Setcanseeplayer true)
      (if (not (Variables|Default|Getisdead))
        (AI|AIMoveTo self "0, 0, 0" _asbp_first_person_character_3 5.0 false
          (:OnSuccess
            (Sprite|SetFlipbook (Variables|Default|GetPaperFlipbook) "/Game/sprites/EnemySprites/DogAttack.DogAttack")
            (bind _asbp_first_person_character_4 (Utilities|Casting|CastToBP_FirstPersonCharacter (Game|GetPlayerCharacter 0)))
            (Game|Damage|ApplyDamage _asbp_first_person_character_4 1.0 0 0)))))))

(event Custom|Random%20Raom
  ;[1 1 1] Random Roam
  (if (not (Variables|Default|Getisdead))
    (AI|AIMoveTo self (.RandomLocation (AI|Navigation|GetRandomReachablePointinRadius (Transformation|GetActorLocation) 2e+03 0 0)) 0 5.0 false
      (:then
        (Utilities|FlowControl|Delay 4.0)
        (if (not (Variables|Default|GetIsAttacking))
          (CallFunction|RandomRaom))))))

(event EventBeginPlay
  (Components|Tick|SetComponentTickEnabled (Variables|Default|GetPaperFlipbook) true)
  (CallFunction|RandomRaom)
  (if (Variables|Default|Getcanseeplayer)
    (if (not (Variables|Default|Getisdead))
      (Transformation|SetActorRotation (Math|Rotator|MakeRotator 0.0 0.0 (.yaw (Math|Rotator|FindLookatRotation (Transformation|GetActorLocation) (Transformation|GetActorLocation (Game|GetPlayerCharacter 0)))))))))

(event EventTick
  (params (DeltaSeconds :type Float%20%28single-precision%29)))

(event Game|Damage|EventAnyDamage
  (params (Damage :type Float%20%28single-precision%29) (DamageType :type Damage%20Type%20Object%20Reference) (InstigatedBy :type Controller%20Object%20Reference) (DamageCauser :type Actor%20Object%20Reference))
  (bind _paperflipbook (Variables|Default|GetPaperFlipbook))
  ;[1 1 1] death Behaivour
  (Utilities|FlowControl|DoOnce false
    (:Completed
      (Components|Activation|Deactivate (Variables|Character|GetCharacterMovement))
      (Sprite|SetFlipbook _paperflipbook (Variables|Default|GetBeforeDeath))
      (Components|Timeline|SetLooping _paperflipbook false)
      (Utilities|FlowControl|Delay (Class|PaperFlipbookComponent|GetFlipbookLength (Variables|Default|GetPaperFlipbook)))
      (Sprite|SetFlipbook _paperflipbook (Variables|Default|GetDeathAnim))
      (Variables|Default|Setisdead true)
      (Collision|SetCollisionEnabled (Variables|Collision|GetCapsuleComponent) "NoCollision"))))

(fn ConstructionScript)